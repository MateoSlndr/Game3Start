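; GM_SaveLoad is a game mode that loads and saves player stats through an SG_PlayerStats save object.
; On BeginPlay it loads the "PlayerSave" slot and copies Stamina to BP_ThirdPersonCharacter, or creates a new save object if none exists.
; SavePlayerStats writes that object without updating its values and uses an empty slot name, unlike loading.
; Debug prints report progress; a misspelled slot check is left unwired.
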(event `Load Player Stats`
  (bind _returnvalue (`GameplayStatics.DoesSaveGameExist` "PlayerSave"))
  (if _returnvalue
    (bind _returnvalue_2 (`GameplayStatics.LoadGameFromSlot` "PlayerSave"))
    (bind _assg_player_stats (cast `/Game/Blueprints/SavingLoading/SG_PlayerStats` _returnvalue_2))
    (set `self.SG_PlayerStats` _assg_player_stats)
    (bind _asbp_third_person_character (cast `/Game/ThirdPerson/Blueprints/BP_ThirdPersonCharacter` (`GameplayStatics.GetPlayerCharacter` 0)))
    (set `/Game/ThirdPerson/Blueprints/BP_ThirdPersonCharacter.Stamina` (`/Game/Blueprints/SavingLoading/SG_PlayerStats.Stamina` (`self.SG_PlayerStats`)) _asbp_third_person_character)
    (`KismetSystemLibrary.PrintString` "PlayerStats have been loaded" true true (struct :`R` 1.0 :`G` 0.435674 :`A` 1.0) 8.0)
    (else
      (bind _returnvalue_3 (`GameplayStatics.CreateSaveGameObject` "/Game/Blueprints/SavingLoading/SG_PlayerStats.SG_PlayerStats_C"))
      (set `self.SG_PlayerStats` _returnvalue_3))))

(event `self.ReceiveBeginPlay`
  (`KismetSystemLibrary.PrintString` "Loading the SaveLoad game mode" true true (struct :`R` 1.0 :`G` 0.298415 :`A` 1.0) 10.0)
  (`self.Load Player Stats`))

(event `Save Player Stats`
  (bind _returnvalue (`GameplayStatics.SaveGameToSlot` (`self.SG_PlayerStats`)))
  (if _returnvalue
    (`KismetSystemLibrary.PrintText` "Player stats written to game save file" true true (struct :`R` 0.035832 :`G` 1.0 :`A` 1.0) 5.0)
    (else
      (`KismetSystemLibrary.PrintText` "Player stats NOT be written to game save file" true true (struct :`R` 0.690625 :`B` 0.02824 :`A` 1.0) 5.0))))

(fn `UserConstructionScript`)