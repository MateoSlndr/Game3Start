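; Speed boost item that is carried like a weapon and changes the player character's walk speed.
; Pickup attaches it to the given skeletal mesh's weapon socket and disables booster collision; Drop detaches it, restores collision and simulates physics briefly.
; Primary and secondary use set fast or normal max walk speed on player 0's BP_ThirdPersonCharacter, regardless of holder.
; Drop leaves the current speed unchanged.
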(event `/Game/Blueprints/BPI_Item.Drop`
  (bind _speedbooster (`self.SpeedBooster`))
  (`self.K2_DetachFromActor` "KeepWorld" "KeepWorld" "KeepWorld")
  (`PrimitiveComponent.SetSimulatePhysics` _speedbooster true)
  (`PrimitiveComponent.SetCollisionEnabled` _speedbooster "QueryAndPhysics")
  (`KismetSystemLibrary.Delay` 2.0)
  (`PrimitiveComponent.SetSimulatePhysics` (`self.SpeedBooster`) false))

(event `/Game/Blueprints/BPI_Item.Pickup`
  (params (SkeletalMesh :type "SkeletalMeshComponent Object Reference"))
  (`KismetSystemLibrary.PrintText` (`|FormatText` "{name} is getting picked up and attached to {mesh}" "Machine Gun" SkeletalMesh) true true (struct :`R` 1.0 :`B` 0.941381 :`A` 1.0))
  (`self.K2_AttachToComponent` SkeletalMesh "Weapon_Socket" "SnapToTarget" "SnapToTarget" "SnapToTarget")
  (`PrimitiveComponent.SetCollisionEnabled` (`self.SpeedBooster`) "NoCollision"))

(event `/Game/Blueprints/BPI_Item.UsePrimary`
  (bind _asbp_third_person_character (cast `/Game/ThirdPerson/Blueprints/BP_ThirdPersonCharacter` (`GameplayStatics.GetPlayerCharacter` 0)))
  (set `CharacterMovementComponent.MaxWalkSpeed` 2000.0 (`Character.CharacterMovement` _asbp_third_person_character))
  (`KismetSystemLibrary.PrintText` "So Fast!" true true (struct :`R` 0.127438 :`G` 1.0 :`A` 1.0)))

(event `/Game/Blueprints/BPI_Item.UseSecondary`
  (bind _asbp_third_person_character (cast `/Game/ThirdPerson/Blueprints/BP_ThirdPersonCharacter` (`GameplayStatics.GetPlayerCharacter` 0)))
  (set `CharacterMovementComponent.MaxWalkSpeed` 600.0 (`Character.CharacterMovement` _asbp_third_person_character))
  (`KismetSystemLibrary.PrintText` "Normal Speed" true true (struct :`R` 0.127438 :`G` 1.0 :`A` 1.0)))

(fn `UserConstructionScript`)