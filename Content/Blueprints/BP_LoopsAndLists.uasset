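; Demo Blueprint for loops and arrays that prints colored debug messages on screen, starting at BeginPlay.
; DelayLoop prints and increments a counter, waits one second, calls PrintColors, then calls itself to repeat indefinitely.
; PrintColors shuffles the Textcolor array and loops over it, printing a random color index in a random color each pass rather than using the loop element.
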(event `self.ReceiveBeginPlay`
  (`KismetSystemLibrary.PrintString` "Loops and lists is active")
  (`self.Delay Loop`))

(event `Delay Loop`
  (`KismetSystemLibrary.PrintString` (`KismetStringLibrary.Concat_StrStr` "Starting Delay Loop #" (`KismetStringLibrary.Conv_IntToString` (`self.DelayLoopCounter`))))
  (`/Engine/EditorBlueprintResources/StandardMacros.IncrementInt` (`self.DelayLoopCounter`)
    (:`  `
      (`KismetSystemLibrary.Delay` 1.0)
      (`self.Print Colors`)
      (`self.Delay Loop`))))

(event `Print Colors`
  (bind _textcolor (`self.Textcolor`))
  (bind (_outitem _outindex) (`KismetArrayLibrary.Array_Random` (`|MakeArray` (struct :`G` 0.145406 :`B` 1.0 :`A` 1.0) (struct :`R` 0.183392 :`G` 1.0 :`A` 1.0) (struct :`R` 1.0 :`G` 0.026021 :`A` 1.0) (struct :`R` 1.0 :`G` 0.91165 :`B` 0.00666 :`A` 1.0) :!type "LinearColor Structure")))
  (`KismetArrayLibrary.Array_Shuffle` _textcolor)
  (for _ _textcolor
    (`KismetSystemLibrary.PrintString` (`KismetStringLibrary.Concat_StrStr` "Print Color #" (`KismetStringLibrary.Conv_IntToString` _outindex)) true true _outitem))
  (`KismetSystemLibrary.PrintString` "We are done Printing Colors!"))

(fn `UserConstructionScript`)