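; BP_Jumper is a held item that launches the player character upward or slams them down.
; Pickup attaches it to the mesh's Weapon_Socket without collision, and Drop detaches it with briefly simulated physics.
; Primary use launches upward and clears CanUse, which resets only after a delay started by another press during cooldown.
; Secondary use applies a downward fast-fall launch with no cooldown.
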(event `/Game/Blueprints/BPI_Item.Drop`
  (bind _jumper_body (`self.Jumper Body`))
  (`self.K2_DetachFromActor` "KeepWorld" "KeepWorld" "KeepWorld")
  (`PrimitiveComponent.SetSimulatePhysics` _jumper_body true)
  (`PrimitiveComponent.SetCollisionEnabled` _jumper_body "QueryAndPhysics")
  (`KismetSystemLibrary.Delay` 2.0)
  (`PrimitiveComponent.SetSimulatePhysics` (`self.Jumper Body`) false))

(event `/Game/Blueprints/BPI_Item.Pickup`
  (params (SkeletalMesh :type "SkeletalMeshComponent Object Reference"))
  (`KismetSystemLibrary.PrintText` (`|FormatText` "{name} is getting picked up and attached to {mesh}" "Machine Gun" SkeletalMesh) true true (struct :`R` 1.0 :`B` 0.941381 :`A` 1.0))
  (`self.K2_AttachToComponent` SkeletalMesh "Weapon_Socket" "SnapToTarget" "SnapToTarget" "SnapToTarget")
  (`PrimitiveComponent.SetCollisionEnabled` (`self.Jumper Body`) "NoCollision"))

(event `/Game/Blueprints/BPI_Item.UsePrimary`
  (if (`self.Can Use`)
    (bind _asbp_third_person_character (cast `/Game/ThirdPerson/Blueprints/BP_ThirdPersonCharacter` (`GameplayStatics.GetPlayerCharacter` 0)))
    (`Character.LaunchCharacter` _asbp_third_person_character (0.0 0.0 1500.0) false false)
    (set `self.Can Use` false)
    (else
      (`KismetSystemLibrary.PrintString` "Cool Down")
      (`KismetSystemLibrary.Delay` 1.5)
      (set `self.Can Use` true))))

(event `/Game/Blueprints/BPI_Item.UseSecondary`
  (bind _asbp_third_person_character (cast `/Game/ThirdPerson/Blueprints/BP_ThirdPersonCharacter` (`GameplayStatics.GetPlayerCharacter` 0)))
  (`Character.LaunchCharacter` _asbp_third_person_character (0.0 0.0 -5000.0) false false)
  (`KismetSystemLibrary.PrintText` "Fast Fall"))

(fn `UserConstructionScript`)