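; Machine gun weapon actor that can be picked up, dropped and used with primary and secondary actions.
; Pickup attaches it to the given skeletal mesh's Weapon_Socket and disables body collision.
; Drop detaches it, restores collision and simulates physics briefly before freezing the body.
; Primary use only prints placeholder firing text, while secondary use toggles zoom by changing the third-person character's camera boom length.
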(event `/Game/Blueprints/BPI_Item.Drop`
  (bind _machinegunbody (`self.MachineGunBody`))
  (`self.K2_DetachFromActor` "KeepWorld" "KeepWorld")
  (`PrimitiveComponent.SetSimulatePhysics` _machinegunbody true)
  (`PrimitiveComponent.SetCollisionEnabled` _machinegunbody "QueryAndPhysics")
  (`KismetSystemLibrary.Delay` 2.0)
  (`PrimitiveComponent.SetSimulatePhysics` (`self.MachineGunBody`) false))

(event `/Game/Blueprints/BPI_Item.UseSecondary`
  (`KismetSystemLibrary.PrintText` "Zooming in")
  (bind _asbp_third_person_character (cast `/Game/ThirdPerson/Blueprints/BP_ThirdPersonCharacter` (`GameplayStatics.GetPlayerCharacter` 0)))
  (if (`self.IsZoomed`)
    (bind _cameraboom (`/Game/ThirdPerson/Blueprints/BP_ThirdPersonCharacter.CameraBoom` _asbp_third_person_character))
    (set `SpringArmComponent.TargetArmLength` 300.0 _cameraboom)
    (set `self.IsZoomed` false)
    (else
      (set `SpringArmComponent.TargetArmLength` 150.0 _cameraboom)
      (set `self.IsZoomed` true))))

(event `/Game/Blueprints/BPI_Item.UsePrimary`
  (`KismetSystemLibrary.PrintText` "Bang Bang"))

(event `/Game/Blueprints/BPI_Item.Pickup`
  (params (SkeletalMesh :type "SkeletalMeshComponent Object Reference"))
  ; Pickup Funciton
  (`KismetSystemLibrary.PrintText` (`|FormatText` "{name} is getting picked up and attached to {mesh}" "Machine Gun" SkeletalMesh) true true (struct :`R` 1.0 :`B` 0.941381 :`A` 1.0))
  (`self.K2_AttachToComponent` SkeletalMesh "Weapon_Socket" "SnapToTarget" "SnapToTarget" "KeepRelative")
  (`PrimitiveComponent.SetCollisionEnabled` (`self.MachineGunBody`) "NoCollision"))

(fn `UserConstructionScript`)