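; BP_EnemyBase is an enemy character that provides attack, aggro, walk speed and patrol functions for AI logic such as BTT_SetSpeed.
; Attack plays a kick montage and calls AttackFinished on completion or interruption.
; Gaining aggro swaps the mesh to a red material, and losing it restores the material cached at BeginPlay.
; GetNextPatrolPointLocation steps along the assigned PatrolRoute spline, reversing direction at either end to ping-pong.
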(event `self.ReceiveBeginPlay`
  (set `self.Original Material` (`PrimitiveComponent.GetMaterial` (`self.Mesh`) 0)))

(event `Attack`
  (`KismetSystemLibrary.PrintString` "Attacking player!")
  (`|PlayMontage` (`self.Mesh`) "/Game/CloseCombatAnimSet/Animations/InPlace/Attacks/NinjaWheelKick_Montage.NinjaWheelKick_Montage"
    (:`OnCompleted`
      _)
    (:`OnInterrupted`
      _))
  (`self.AttackFinished`))

(event `Get Aggro`
  (`PrimitiveComponent.SetMaterial` (`self.Mesh`) 0 "/AnimationSharing/AnimSharingRed.AnimSharingRed")
  (set `self.Aggroed` true))

(event `Lose Aggro`
  (`PrimitiveComponent.SetMaterial` (`self.Mesh`) 0 (`self.Original Material`))
  (set `self.Aggroed` false))

(event `SetWalkSpeed`
  (params (`New Speed` :type "Float (single-precision)"))
  (set `CharacterMovementComponent.MaxWalkSpeed` `New Speed` (`self.CharacterMovement`)))

(fn `GetNextPatrolPointLocation`
  (returns (Location :type "Vector Structure"))
  (`/Engine/EditorBlueprintResources/StandardMacros.IsValid` (`self.Patrol Route`)
    (:`Is Valid`
      (set `self.Patrol Point index` (+ (`self.Patrol Point index`) (`self.PatraolRouteDirection`)))
      (if (or (>= (`self.Patrol Point index`) (- (`SplineComponent.GetNumberOfSplinePoints` (`/Game/Blueprints/BP_PatrolRoute.Spline` (`self.Patrol Route`))) 1)) (<= (`self.Patrol Point index`) 0))
        (set `self.PatraolRouteDirection` (* (`self.PatraolRouteDirection`) -1)))
      (return (`SplineComponent.GetLocationAtSplinePoint` (`/Game/Blueprints/BP_PatrolRoute.Spline` (`self.Patrol Route`)) (`self.Patrol Point index`) "World")))
    (:`Is Not Valid`
      (`KismetSystemLibrary.PrintString` "No Patrol Route Assigned"))))

(fn `UserConstructionScript`)